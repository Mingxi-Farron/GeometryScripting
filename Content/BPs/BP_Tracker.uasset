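; BP_Tracker is a moving actor that feeds the world positions of four corner points to a Mesh reference.
; Each Tick moves the root around a time-driven sine/cosine circle about the world origin and spins the Plane in yaw by a fixed per-frame step.
; GetLocations then gathers the 00, 10, 11 and 01 component locations in perimeter order into Buffer and assigns it to the Mesh's Next variable.
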(event EventBeginPlay)

(event Collision|EventActorBeginOverlap
  (params (OtherActor :type Actor%20Object%20Reference)))

(event EventTick
  (params (DeltaSeconds :type Float%20%28single-precision%29))
  (bind _returnvalue (Actor|GetGameTimeSinceCreation))
  (bind _returnvalue_2 (* _returnvalue 3e+01))
  (Transformation|SetWorldLocation (Variables|Default|GetDefaultSceneRoot) (Math|Vector|MakeVector (* (Math|Trig|Sin(Degrees) _returnvalue_2) 3e+02) (* (Math|Trig|Cos(Degrees) _returnvalue_2) 3e+02) 0.0) false false)
  (Transformation|AddLocalRotation (Variables|Default|GetPlane) (Math|Rotator|MakeRotator 0.0 0.0 1.0) false false)
  (CallFunction|GetLocations))

(fn ConstructionScript)

(fn GetLocations
  (Utilities|Array|Add (LocalVariables|GetBuffer) (Transformation|GetWorldLocation (Variables|Default|Get0_0)))
  (Utilities|Array|Add (LocalVariables|GetBuffer) (Transformation|GetWorldLocation (Variables|Default|Get1_0)))
  (Utilities|Array|Add (LocalVariables|GetBuffer) (Transformation|GetWorldLocation (Variables|Default|Get1_1)))
  (Utilities|Array|Add (LocalVariables|GetBuffer) (Transformation|GetWorldLocation (Variables|Default|Get0_1)))
  (Variables|/Game/BPs/BP_DynamicGenerative.BP_DynamicGenerative_C|SetNext (Variables|Default|GetMesh) (LocalVariables|GetBuffer)))