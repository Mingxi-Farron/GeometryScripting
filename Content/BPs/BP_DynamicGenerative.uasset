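; BP_DynamicGenerative is a Geometry Script generated mesh Blueprint that procedurally builds an organic, noise-distorted swept shape.
; On rebuild, it sweeps the Vertices polygon along Path, applies Perlin noise, then passes the mesh to Smoothing.
; Smoothing applies PN tessellation, iterative smoothing and normal recomputation.
; Unconnected experimental chains for a texture-displaced disc and a revolved polygon remain in the graph but never run.
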(event Events|EventOnRebuildGeneratedMesh
  (params (TargetMesh :type Dynamic%20Mesh%20Object%20Reference))
  (bind _returnvalue (Class|GeometryScriptLibraryMeshPrimitiveFunctions|AppendSimpleSweptPolygon TargetMesh (Utilities|Struct|MakeGeometryScriptPrimitiveOptions "PerFace" false "Uniform") (Math|Transform|MakeTransform "0, 0, 0" "0, 0, 0" "1.000000,1.000000,1.000000") (Variables|Default|GetVertices) (Variables|Default|GetPath) false true 1.0 1.0 0))
  (bind _returnvalue_2 (Class|GeometryScriptLibraryMeshDeformFunctions|ApplyPerlinNoisetoMesh :TargetMesh _returnvalue :Options (Utilities|Struct|MakeGeometryScriptPerlinNoiseOptions (Utilities|Struct|MakeGeometryScriptPerlinNoiseLayerOptions 2e+01 0.25 "0.000000,0.000000,0.000000" 0) true "FullMeshSelection") :Debug 0))
  (CallFunction|Smoothing _returnvalue_2))

(fn ConstructionScript)

(fn Smoothing
  (params (Mesh :type Dynamic%20Mesh%20Object%20Reference))
  (bind _returnvalue (Class|GeometryScriptLibraryMeshSubdivideFunctions|ApplyPNTessellation Mesh (Utilities|Struct|MakeGeometryScriptPNTessellateOptions true) 3 0))
  (bind _returnvalue_2 (Class|GeometryScriptLibraryMeshDeformFunctions|ApplyIterativeSmoothingtoMesh :TargetMesh _returnvalue :Debug 0))
  (bind _returnvalue_3 (GeometryScript|Normals|RecomputeNormals :TargetMesh _returnvalue_2 :Debug 0))
  (return _returnvalue_3))